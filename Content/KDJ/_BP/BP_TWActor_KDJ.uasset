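; BP_TWActor_KDJ is an actor that turns the game window into a transparent, topmost, click-through desktop overlay.
; On BeginPlay it enables input, makes the window transparent via GDI, then turns on topmost and click-through modes.
; A keyboard hook on F2 is created for cancelling click-through and is released on EndPlay.
; Number keys toggle click-through and topmost modes on and off.
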(event `self.ReceiveBeginPlay`
  (`self.EnableInput` (`GameplayStatics.GetPlayerController` 0))
  (`self.MakeTransparentWindow` "GDI")
  (`self.CreateHookForCancelClickThrough` "Keyboard_VK_F2")
  (`self.SetWindowsTopMode` true)
  (`self.SetWindowsClickThrough` true))

(event `Key|One`
  (params (Key :type "Key Structure"))
  (:`Pressed`
    (`self.SetWindowsClickThrough` true)))

(event `Key|Two`
  (params (Key :type "Key Structure"))
  (:`Pressed`
    (`self.SetWindowsClickThrough` false)))

(event `self.ReceiveEndPlay`
  (params (EndPlayReason :type "EEndPlayReason Enum" :default "Destroyed"))
  (`self.CancelHook`))

(event `Key|Three`
  (params (Key :type "Key Structure"))
  (:`Pressed`
    (`self.SetWindowsTopMode` true)))

(event `Key|Four`
  (params (Key :type "Key Structure"))
  (:`Pressed`
    (`self.SetWindowsTopMode` false)))

(fn `UserConstructionScript`)