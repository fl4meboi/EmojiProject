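; Player controller for the emoji feature that maps keyboard keys to spawning emojis and quitting.
; On BeginPlay it caches the BP_EmojiManager found in the level, shows the mouse cursor and switches input to Game and UI.
; S triggers SpawnEmoji, C triggers CenterSpawnEmoji and Escape quits the game.
; The InputActionSpawn event is an empty stub.
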(event `InputActionSpawn`)

(event `self.ReceiveBeginPlay`
  (bind _returnvalue (`GameplayStatics.GetActorOfClass` "/Game/KDJ/_BP/BP_EmojiManager.BP_EmojiManager_C"))
  (set `self.EmojiManager` _returnvalue)
  (set `self.bShowMouseCursor` true)
  (`WidgetBlueprintLibrary.SetInputMode_GameAndUIEx` self null))

(event `Key|S`
  (params (Key :type "Key Structure"))
  (:`Pressed`
    (`self.SpawnEmoji`)))

(event `Key|Escape`
  (params (Key :type "Key Structure"))
  (:`Pressed`
    (`KismetSystemLibrary.QuitGame` null "Quit")))

(event `Key|C`
  (params (Key :type "Key Structure"))
  (:`Pressed`
    (`self.CenterSpawnEmoji`)))

(fn `UserConstructionScript`)