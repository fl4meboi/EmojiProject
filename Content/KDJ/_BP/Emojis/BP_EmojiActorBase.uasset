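; Base actor for a short-lived emoji shown as a Paper2D flipbook that fades out and destroys itself.
; Tick passes through a 1.2-second delay, then plays a Fade timeline that drives the flipbook material's "Fade" scalar parameter and prints the value.
; Timeline updates also feed a 2.5-second delay, after which it calls DestroyEvent and destroys the actor.
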(event `self.ReceiveBeginPlay`)

(event `self.ReceiveTick`
  (params (DeltaSeconds :type "Float (single-precision)"))
  (cast `MaterialInstanceDynamic` (`PrimitiveComponent.GetMaterial` (`self.PaperFlipbook`) 0)
    (:`then`
      _)
    (:`CastFailed`
      _))
  (`KismetSystemLibrary.Delay` 1.2)
  (bind (_direction _fadevalue) (`Timeline|Fade`)
    (:`Update`
      (`KismetSystemLibrary.PrintString` (`KismetStringLibrary.Conv_DoubleToString` _fadevalue))
      (`MeshComponent.SetScalarParameterValueOnMaterials` (`self.PaperFlipbook`) "Fade" _fadevalue)
      (`KismetSystemLibrary.Delay` 2.5)
      (`self.DestroyEvent`)
      (`self.K2_DestroyActor`))))

(fn `UserConstructionScript`)